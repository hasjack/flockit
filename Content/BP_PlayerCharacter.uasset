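; Player character Blueprint that turns input axes into movement and camera-independent yaw control.
; LeftRight and ForwardBackward add movement input along the actor's right and forward vectors, scaled by a Speed variable.
; The Stop axis halts the character movement component immediately at full value, and Turn adds controller yaw at reduced sensitivity.
; The construction script is empty.
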(event Input|AxisEvents|InputAxisLeftRight
  (params (AxisValue :type Float%20%28single-precision%29))
  (Pawn|Input|AddMovementInput (Transformation|GetActorRightVector) (* (Variables|Default|Getspeed) AxisValue) false))

(event Input|AxisEvents|InputAxisStop
  (params (AxisValue :type Float%20%28single-precision%29))
  (if (== AxisValue 1.0)
    (Components|Movement|StopMovementImmediately (Variables|Character|GetCharacterMovement))))

(event Input|AxisEvents|InputAxisTurn
  (params (AxisValue :type Float%20%28single-precision%29))
  (Pawn|Input|AddControllerYawInput (* AxisValue 0.1)))

(event Input|AxisEvents|InputAxisForwardBackward
  (params (AxisValue :type Float%20%28single-precision%29))
  (Pawn|Input|AddMovementInput (Transformation|GetActorForwardVector) (* (Variables|Default|Getspeed) AxisValue) false))

(fn ConstructionScript)