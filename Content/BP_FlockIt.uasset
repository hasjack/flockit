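; Flocking visualizer actor that spawns the initial species and renders their organisms as instanced static meshes.
; BeginPlay creates one shadowless, collisionless instanced mesh component per species, a cone for "Torpedo"-prefixed names or else a sphere, tinted with its debug color.
; Each Tick copies velocity-oriented organism transforms to the instances, using cumulative populations to map global IDs to component and local index.
; A batch-update call is present but unconnected.
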(event EventBeginPlay
  (bind _populations (Variables|Default|Getpopulations))
  (for (_array_element _array_index) (Variables|Default|GetInitialSpecies)
    (Class|FlockManager|SpawnSpecies (.species _array_element) (.count _array_element))
    (bind _returnvalue (AddComponent|AddInstancedStaticMeshComponent false))
    (bind _name (CallFunction|GetSpeciesName (.species _array_element)))
    (if (Utilities|String|StartsWith (Utilities|String|ToString(Name) _name) "Torpedo")
      (Components|StaticMesh|SetStaticMesh _returnvalue "/Engine/BasicShapes/Cone.Cone")
      (else
        (Components|StaticMesh|SetStaticMesh _returnvalue "/Engine/BasicShapes/Sphere.Sphere")))
    (Rendering|SetCastShadow _returnvalue false)
    (Collision|SetCollisionEnabled _returnvalue "NoCollision")
    (bind _returnvalue_2 (Rendering|Material|CreateDynamicMaterialInstance _returnvalue 0 "/Engine/BasicShapes/BasicShapeMaterial.BasicShapeMaterial" "" :!class /Script/Engine.PrimitiveComponent))
    (bind _color (CallFunction|GetSpeciesColor (.species _array_element)))
    (Rendering|Material|SetVectorParameterValue _returnvalue_2 "Color" _color :!class /Script/Engine.MaterialInstanceDynamic)
    (Utilities|Array|Add (Variables|Default|GetISMeshes) _returnvalue)
    (if (== _array_index 0)
      (Utilities|Array|Add _populations (.count _array_element))
      (else
        (Utilities|Array|Add _populations (+ (.count _array_element) (Utilities|Array|Get(acopy) _populations (- _array_index 1)))))))
  (for (_array_element_2 _array_index_2) (Class|FlockManager|GetOrganismWorldTransforms (Variables|Default|GetInstance%20Scale) true "PositiveZ")
    (bind _index (CallFunction|GetISMeshIndex _array_index_2))
    (Components|InstancedStaticMesh|AddInstance (Utilities|Array|Get(acopy) (Variables|Default|GetISMeshes) _index) _array_element_2 true)))

(event EventTick
  (params (DeltaSeconds :type Float%20%28single-precision%29))
  (for (_array_element _array_index) (Class|FlockManager|GetOrganismWorldTransforms (Variables|Default|GetInstance%20Scale) true "PositiveZ")
    (bind _index (CallFunction|GetISMeshIndex _array_index))
    (if (== _index 0)
      (Components|InstancedStaticMesh|UpdateInstanceTransform (Utilities|Array|Get(acopy) (Variables|Default|GetISMeshes) _index) _array_index _array_element true false false)
      (else
        (Components|InstancedStaticMesh|UpdateInstanceTransform (Utilities|Array|Get(acopy) (Variables|Default|GetISMeshes) _index) (- _array_index (Utilities|Array|Get(acopy) (Variables|Default|Getpopulations) (- _index 1))) _array_element true false false)))))

(fn ConstructionScript)

(fn GetISMeshIndex
  (params (id :type Integer))
  (bind (_array_element _array_index) (Utilities|Array|ForEachLoopwithBreak (Variables|Default|Getpopulations) :!label _label)
    (:LoopBody
      (if (< id _array_element)
        (goto _label Break)))
    (:Completed
      (return _array_index))))

(fn GetSpeciesColor
  (params (species :type Org%20Type%20Structure))
  (return (.debugcolor species)))

(fn GetSpeciesName
  (params (species :type Org%20Type%20Structure))
  (return (.speciesname species)))